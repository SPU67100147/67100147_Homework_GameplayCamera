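; BP_Button is an interactable button that shows a "Press Button" prompt at the Button component's location.
; On interact, it sets a motion warping target 70 units from the button toward the interacter, yawed to face it.
; It then plays a left-hand press montage on the interacter and clears the IsInteract flag when the montage completes or is interrupted.
; The graph itself triggers no effect from the press.
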(event EventBeginPlay
  (|CallParentFunction) ; This node is disabled and will not be called.\nDrag off pins to build functionality.
)

(event Collision|EventActorBeginOverlap
  (params (OtherActor :type Actor%20Object%20Reference))
  (|CallParentFunction OtherActor) ; This node is disabled and will not be called.\nDrag off pins to build functionality.
)

(event EventTick
  (params (DeltaSeconds :type Float%20%28single-precision%29))
  (|CallParentFunction DeltaSeconds) ; This node is disabled and will not be called.\nDrag off pins to build functionality.
)

(event EventOnInteract
  (params (Interacter :type BP%20Third%20Person%20Character%20Object%20Reference))
  (bind _returnvalue (Transformation|GetActorLocation Interacter))
  (bind _self self)
  (bind _returnvalue_2 (Transformation|GetActorLocation _self))
  (bind _returnvalue_3 (- _returnvalue _returnvalue_2))
  (bind _returnvalue_4 (Math|Vector|Normalize _returnvalue_3))
  (bind _returnvalue_5 (* _returnvalue_4 -1.0))
  (bind (_x _y) (Math|Vector|BreakVector _returnvalue_5))
  (|CallParentFunction Interacter)
  (Class|MotionWarpingComponent|AddorUpdateWarpTargetfromLocationandRotation (Variables|/Game/Blueprints/ThirdPerson/Blueprints/BP_ThirdPersonCharacter.BP_ThirdPersonCharacter_C|GetMotionWarping Interacter) "InteractTarget" (+ (* _returnvalue_4 7e+01) _returnvalue_2) (Math|Rotator|MakeRotfromX (Math|Vector|MakeVector _x _y 0.0)))
  (Animation|Montage|PlayMontage (Variables|/Script/Engine.Character|GetMesh Interacter) "/Game/Assets/Animations/AM_PressButton_L.AM_PressButton_L"
    (:OnCompleted
      _)
    (:OnInterrupted
      _))
  (Variables|Default|SetIsInteract false))

(fn ConstructionScript
  (|CallParentFunction))

(fn GetInteractText
  (return "Press Button"))

(fn GetInteractTextLocation
  (return (Transformation|GetWorldLocation (Variables|Default|GetButton))))